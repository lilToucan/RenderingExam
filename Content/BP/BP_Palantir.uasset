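; BP_Palantir is an actor whose Sphere component shows a palantír material that gradually changes its wear over time.
; BeginPlay creates a dynamic instance of MI_Palantir on the Sphere and stores it.
; Each Tick lowers the instance's WearContrast and raises its WearAmount by a fixed step, unclamped and not scaled by delta time, so the speed depends on frame rate.
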(event EventBeginPlay
  (bind _returnvalue (Rendering|Material|CreateDynamicMaterialInstance (Variables|Default|GetSphere) 0 "/Game/Materials_LEZIONI/MI_Palantir.MI_Palantir" "None" :!class /Script/Engine.PrimitiveComponent))
  (Variables|Default|SetMIDR _returnvalue))

(event EventTick
  (params (DeltaSeconds :type Float%20%28single-precision%29))
  (bind _returnvalue (Rendering|Material|GetScalarParameterValue (Variables|Default|GetMIDR) "WearContrast" :!class /Script/Engine.MaterialInstanceDynamic))
  (Rendering|Material|SetScalarParameterValue (Variables|Default|GetMIDR) "WearContrast" (- _returnvalue 0.001) :!class /Script/Engine.MaterialInstanceDynamic)
  (bind _returnvalue_2 (Rendering|Material|GetScalarParameterValue (Variables|Default|GetMIDR) "WearAmount" :!class /Script/Engine.MaterialInstanceDynamic))
  (Rendering|Material|SetScalarParameterValue (Variables|Default|GetMIDR) "WearAmount" (+ _returnvalue_2 0.001) :!class /Script/Engine.MaterialInstanceDynamic))

(fn ConstructionScript)
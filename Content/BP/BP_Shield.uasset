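; Energy shield actor that changes its look as the player pawn gets closer.
; BeginPlay creates a dynamic material on the sphere, enables player input and caches the starting rim color.
; Each Tick, inverse player distance drives the contact start parameter and blends contact color from that cached color toward green.
; Pressing B turns the rim magenta without updating the cached color.
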(event EventBeginPlay
  (bind _returnvalue (Rendering|Material|CreateDynamicMaterialInstance (Variables|Default|GetSphere) 0 "/Game/Materials_LEZIONI/MI_EnergyShield.MI_EnergyShield" "None" :!class /Script/Engine.PrimitiveComponent))
  (Variables|Default|SetMIDR _returnvalue)
  (Input|EnableInput (Game|GetPlayerController 0))
  (bind _returnvalue_2 (Rendering|Material|GetVectorParameterValue (Variables|Default|GetMIDR) "RimColor" :!class /Script/Engine.MaterialInstanceDynamic))
  (Variables|Default|SetStartColor _returnvalue_2))

(event EventTick
  (params (DeltaSeconds :type Float%20%28single-precision%29))
  (bind _returnvalue (Game|Player|GetPlayerPawn 0))
  (bind _returnvalue_2 (Transformation|GetActorLocation))
  (bind _returnvalue_3 (Transformation|GetActorLocation _returnvalue))
  (bind _returnvalue_4 (Math|Vector|Distance(Vector) _returnvalue_3 _returnvalue_2))
  (Rendering|Material|SetScalarParameterValue (Variables|Default|GetMIDR) "ContactStart" (/ -8e+03 _returnvalue_4) :!class /Script/Engine.MaterialInstanceDynamic)
  (Rendering|Material|SetVectorParameterValue (Variables|Default|GetMIDR) "ContactColor" (Math|Color|Lerp(LinearColor) (Variables|Default|GetStartColor) "(R=0.000000,G=1.000000,B=0.026761,A=1.000000)" (/ 1e+02 _returnvalue_4)) :!class /Script/Engine.MaterialInstanceDynamic))

(event Input|KeyboardEvents|B
  (params (Key :type Key%20Structure :default "None"))
  (:Pressed
    (Rendering|Material|SetVectorParameterValue (Variables|Default|GetMIDR) "RimColor" "(R=0.919565,G=0.000000,B=1.000000,A=1.000000)" :!class /Script/Engine.MaterialInstanceDynamic)))

(fn ConstructionScript)
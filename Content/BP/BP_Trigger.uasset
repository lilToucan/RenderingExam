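; BP_Trigger is an overlap trigger that changes a wall's color and intensity through a Material Parameter Collection.
; On BeginPlay it enables player input and caches the starting WallColor.
; Overlap raises WallIntensity and sets the color to yellow; leaving zeroes the intensity and restores the cached color.
; While overlapped, the K and L keys switch the color to green or red.
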(event EventBeginPlay
  (Input|EnableInput (Game|GetPlayerController 0))
  (bind _returnvalue (Rendering|Material|GetVectorParameterValue (Variables|Default|GetMPC) (Utilities|Name|MakeLiteralName "WallColor") :!class /Script/Engine.KismetMaterialLibrary))
  (Variables|Default|SetStartColor _returnvalue))

(event Collision|EventActorBeginOverlap
  (params (OtherActor :type Actor%20Object%20Reference))
  (Variables|Default|SetOverlapped true)
  (Rendering|Material|SetScalarParameterValue (Variables|Default|GetMPC) (Utilities|Name|MakeLiteralName "WallIntensity") 1.0 :!class /Script/Engine.KismetMaterialLibrary)
  (Rendering|Material|SetVectorParameterValue (Variables|Default|GetMPC) (Utilities|Name|MakeLiteralName "WallColor") (Variables|Default|GetYellow) :!class /Script/Engine.KismetMaterialLibrary))

(event EventTick
  (params (DeltaSeconds :type Float%20%28single-precision%29)))

(event Collision|EventActorEndOverlap
  (params (OtherActor :type Actor%20Object%20Reference))
  (Variables|Default|SetOverlapped false)
  (Rendering|Material|SetScalarParameterValue (Variables|Default|GetMPC) (Utilities|Name|MakeLiteralName "WallIntensity") 0.0 :!class /Script/Engine.KismetMaterialLibrary)
  (Rendering|Material|SetVectorParameterValue (Variables|Default|GetMPC) (Utilities|Name|MakeLiteralName "WallColor") (Variables|Default|GetStartColor) :!class /Script/Engine.KismetMaterialLibrary))

(event Input|KeyboardEvents|L
  (params (Key :type Key%20Structure :default "None"))
  (:Pressed
    (if (Variables|Default|GetOverlapped)
      (Rendering|Material|SetVectorParameterValue (Variables|Default|GetMPC) (Utilities|Name|MakeLiteralName "WallColor") (Variables|Default|GetRed) :!class /Script/Engine.KismetMaterialLibrary))))

(event Input|KeyboardEvents|K
  (params (Key :type Key%20Structure :default "None"))
  (:Pressed
    (if (Variables|Default|GetOverlapped)
      (Rendering|Material|SetVectorParameterValue (Variables|Default|GetMPC) (Utilities|Name|MakeLiteralName "WallColor") (Variables|Default|GetGreen) :!class /Script/Engine.KismetMaterialLibrary))))

(fn ConstructionScript)
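; BP_Flickerer is a trigger actor that toggles a Material Parameter Collection switch when something overlaps its Box component.
; It sets the scalar parameter "IsOn" to zero on BeginPlay, to one when an overlap starts and back to zero when it ends.
; Overlaps are not filtered by actor type, and any visual response is left to materials reading the collection.
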(event OnComponentBeginOverlap(Box)
  (params (OverlappedComponent :type Primitive%20Component%20Object%20Reference) (OtherActor :type Actor%20Object%20Reference) (OtherComp :type Primitive%20Component%20Object%20Reference) (OtherBodyIndex :type Integer) (bFromSweep :type Boolean) (SweepResult :type Hit%20Result%20Structure%20%28by%20ref%29))
  (Rendering|Material|SetScalarParameterValue (Variables|Default|GetMPC) (Utilities|Name|MakeLiteralName "IsOn") 1.0 :!class /Script/Engine.KismetMaterialLibrary))

(event OnComponentEndOverlap(Box)
  (params (OverlappedComponent :type Primitive%20Component%20Object%20Reference) (OtherActor :type Actor%20Object%20Reference) (OtherComp :type Primitive%20Component%20Object%20Reference) (OtherBodyIndex :type Integer))
  (Rendering|Material|SetScalarParameterValue (Variables|Default|GetMPC) (Utilities|Name|MakeLiteralName "IsOn") 0.0 :!class /Script/Engine.KismetMaterialLibrary))

(event EventBeginPlay
  (Rendering|Material|SetScalarParameterValue (Variables|Default|GetMPC) (Utilities|Name|MakeLiteralName "IsOn") 0.0 :!class /Script/Engine.KismetMaterialLibrary))

(event Collision|EventActorBeginOverlap
  (params (OtherActor :type Actor%20Object%20Reference)))

(event EventTick
  (params (DeltaSeconds :type Float%20%28single-precision%29)))

(fn ConstructionScript)
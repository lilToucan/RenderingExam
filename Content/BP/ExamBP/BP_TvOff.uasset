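; TV actor that shows a random texture on its screen and switches to another when Q is pressed.
; BeginPlay enables player input, creates a dynamic M_TurnTheTvOff material on TvScreen and sets its Texture parameter from the Textures array.
; Q rerolls, retrying next tick until the index differs from PreviousTexture.
; BeginPlay rolls the texture and stored index separately, so they can differ initially.
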(event EventBeginPlay
  (bind _textures (Variables|Default|GetTextures))
  (bind (_outitem _outindex) (Utilities|Array|Random _textures))
  (bind _returnvalue (Rendering|Material|CreateDynamicMaterialInstance (Variables|Default|GetTvScreen) 0 "/Game/MATERIALS_EXAM/M_TurnTheTvOff.M_TurnTheTvOff" "None" :!class /Script/Engine.PrimitiveComponent))
  (Variables|Default|SetDynamicMat _returnvalue)
  (Input|EnableInput (Game|GetPlayerController 0))
  (Rendering|Material|SetTextureParameterValue (Variables|Default|GetDynamicMat) "Texture" _outitem)
  (Variables|Default|SetPreviousTexture _outindex))

(event Collision|EventActorBeginOverlap
  (params (OtherActor :type Actor%20Object%20Reference)))

(event Input|KeyboardEvents|Q
  (params (Key :type Key%20Structure :default "None"))
  (:Pressed
    (Development|PrintString (Utilities|String|ToString(Integer) (Variables|Default|GetPreviousTexture)) :!label _label)
    (bind _outindex (Utilities|Array|Random (Variables|Default|GetTextures)))
    (if (== (Variables|Default|GetPreviousTexture) _outindex)
      (Utilities|FlowControl|DelayUntilNextTick)
      (goto _label)
      (else
        (bind _output_get (Variables|Default|SetPreviousTexture _outindex))
        (Rendering|Material|SetTextureParameterValue (Variables|Default|GetDynamicMat) "Texture" (Utilities|Array|Get(acopy) (Variables|Default|GetTextures) _output_get))))))

(fn ConstructionScript)